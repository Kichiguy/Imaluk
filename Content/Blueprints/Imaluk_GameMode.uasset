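; Game mode for Imaluk, a two-player turn-based board game with black and red pieces.
; On BeginPlay it builds the standard board, currently a single 3x1 piece spawned through a reusable placement helper.
; AddPieceToBoard spawns the current player's placeholder piece on a clickable spot, locks that spot, decrements that player's piece count and passes the turn.
; Blocked placements only print a message, and the touch event is empty.
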(event EventBeginPlay
  (CallFunction|StandardGameBoard))

(event EventActorOnInputTouchBegin
  (params (FingerIndex :type ETouchIndex%20Enum :default "Touch1")))

(fn ConstructionScript)

(fn AddPiecetoBoard
  (params (TouchedPiece :type BP%20Grid%20Piece%20Object%20Reference))
  (bind _sphere (Variables|/Game/Blueprints/BP_grid_piece.BP_grid_piece_C|GetSphere TouchedPiece))
  (bind _returnvalue (Transformation|GetWorldTransform _sphere))
  ;[1 1 1] Check validity of placement
  ;[1 1 1] Check which player's turn and branch
  (if (Variables|/Game/Blueprints/BP_grid_piece.BP_grid_piece_C|GetClickable TouchedPiece)
    (if (Variables|Default|GetBlackPlayerTurn)
      ;[1 1 1] Add the correct piece and assign to selected place on board
      (Game|SpawnActorfromClass "/Game/Assets/Placeholders/PH_Black_Piece.PH_Black_Piece_C" _returnvalue "AlwaysSpawn" TouchedPiece 0)
      (else
        (Game|SpawnActorfromClass "/Game/Assets/Placeholders/PH_Red_Piece.PH_Red_Piece_C" _returnvalue "AlwaysSpawn" TouchedPiece 0)))
    (Variables|/Game/Blueprints/BP_grid_piece.BP_grid_piece_C|SetClickable TouchedPiece false)
    (if (Variables|Default|GetBlackPlayerTurn)
      (CallFunction|UpdateBlackPieces)
      (Variables|Default|SetBlackPlayerTurn false)
      (else
        (CallFunction|UpdateRedPieces)
        (Variables|Default|SetBlackPlayerTurn true)))
    (else
      (Development|PrintString "May not place here"))))

(fn UpdateRedPieces
  (bind _result (Math|Integer|DecrementInt (Variables|Default|GetRedPieceCount))
    (:%20%20
      (Variables|Default|SetRedPieceCount _result))))

(fn UpdateBlackPieces
  (bind _result (Math|Integer|DecrementInt (Variables|Default|GetBlackPieceCount))
    (:%20%20
      (Variables|Default|SetBlackPieceCount _result))))

(fn StandardGameBoard
  (CallFunction|PlacePieceonBoard "/Game/Blueprints/BP_3x1Piece.BP_3x1Piece_C" "100.000000,200.000000, 0" "0, 0, 0"))

(fn PlacePieceonBoard
  (params (BoardPieceClass :type Actor%20Class%20Reference) (Coordinates :type Vector) (Rotation :type Rotator))
  (Game|SpawnActorfromClass BoardPieceClass (Math|Transform|MakeTransform Coordinates Rotation) "AlwaysSpawn" 0 0))